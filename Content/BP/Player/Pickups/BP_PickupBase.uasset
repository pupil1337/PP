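; Base pickup actor that shows a tip widget and offers its item class to a nearby player's weapon manager.
; BeginPlay writes the pickup's text into the BP_PickupTip widget.
; Box overlaps from locally controlled PPCharacters toggle the tip and set or clear PickItem and PickBase on that character's PPWeaponMgr.
; The pickup action itself is not handled here.
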(event OnComponentBeginOverlap(Box)
  (params (OverlappedComponent :type Primitive%20Component%20Object%20Reference) (OtherActor :type Actor%20Object%20Reference) (OtherComp :type Primitive%20Component%20Object%20Reference) (OtherBodyIndex :type Integer) (bFromSweep :type Boolean) (SweepResult :type Hit%20Result%20Structure%20%28by%20ref%29))
  (if (CallFunction|IsLocallyController OtherActor)
    (CallFunction|OnTip true)
    (CallFunction|SetPickItem OtherActor true)))

(event OnComponentEndOverlap(Box)
  (params (OverlappedComponent :type Primitive%20Component%20Object%20Reference) (OtherActor :type Actor%20Object%20Reference) (OtherComp :type Primitive%20Component%20Object%20Reference) (OtherBodyIndex :type Integer))
  (if (CallFunction|IsLocallyController OtherActor)
    (CallFunction|OnTip false)
    (CallFunction|SetPickItem OtherActor false)))

(event Custom|OnTip
  (params (Show :type Boolean))
  (bind _asbp_pickup_tip (Utilities|Casting|CastToBP_PickupTip (UserInterface|GetUserWidgetObject (Variables|Default|GetTip))))
  (Default|OnTip _asbp_pickup_tip Show))

(event Custom|SetPickItem
  (params (Actor :type Actor%20Object%20Reference) (Get :type Boolean))
  (bind _asppcharacter (Utilities|Casting|CastToPPCharacter Actor))
  (if (Utilities|IsValid (Actor|GetComponentbyClass _asppcharacter "/Script/PPGame.PPWeaponMgr"))
    (if Get
      (Variables|/Script/PPGame.PPWeaponMgr|SetPickItem (Actor|GetComponentbyClass _asppcharacter "/Script/PPGame.PPWeaponMgr") (Variables|Default|GetPickClass))
      (Variables|/Script/PPGame.PPWeaponMgr|SetPickBase (Actor|GetComponentbyClass _asppcharacter "/Script/PPGame.PPWeaponMgr") self)
      (else
        (Variables|/Script/PPGame.PPWeaponMgr|SetPickItem (Actor|GetComponentbyClass _asppcharacter "/Script/PPGame.PPWeaponMgr") 0)
        (Variables|/Script/PPGame.PPWeaponMgr|SetPickBase (Actor|GetComponentbyClass _asppcharacter "/Script/PPGame.PPWeaponMgr") 0)))))

(event EventBeginPlay
  (bind _asbp_pickup_tip (Utilities|Casting|CastToBP_PickupTip (UserInterface|GetUserWidgetObject (Variables|Default|GetTip))))
  (Default|TipSetText _asbp_pickup_tip (Variables|Default|GetText)))

(fn ConstructionScript)

(fn IsLocallyController
  (params (Actor :type Actor%20Object%20Reference))
  (bind _asppcharacter (Utilities|Casting|CastToPPCharacter Actor))
  (if (Utilities|IsValid (Pawn|GetController _asppcharacter))
    (return (Pawn|IsLocalPlayerController (Pawn|GetController _asppcharacter)))))