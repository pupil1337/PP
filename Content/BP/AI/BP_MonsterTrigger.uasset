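; Monster trigger volume that detects player characters entering and leaving its collision component.
; Begin and end overlap events cast the other actor to PPCharacter, then call OnPlayerIn or OnPlayerOut only when that character's local role is Authority, keeping notifications server-side for replicated players.
; Each authoritative entry and exit also prints a debug message.
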(event OnComponentEndOverlap(CollisionComponent)
  (params (OverlappedComponent :type Primitive%20Component%20Object%20Reference) (OtherActor :type Actor%20Object%20Reference) (OtherComp :type Primitive%20Component%20Object%20Reference) (OtherBodyIndex :type Integer))
  (bind _asppcharacter (Utilities|Casting|CastToPPCharacter OtherActor))
  (if (Utilities|Enum|Equal(Enum) (Networking|GetLocalRole _asppcharacter) "ROLE_Authority")
    (Class|PPMonsterTrigger|OnPlayerOut _asppcharacter)
    (Development|PrintString "Hello Out")))

(event OnComponentBeginOverlap(CollisionComponent)
  (params (OverlappedComponent :type Primitive%20Component%20Object%20Reference) (OtherActor :type Actor%20Object%20Reference) (OtherComp :type Primitive%20Component%20Object%20Reference) (OtherBodyIndex :type Integer) (bFromSweep :type Boolean) (SweepResult :type Hit%20Result%20Structure%20%28by%20ref%29))
  (bind _asppcharacter (Utilities|Casting|CastToPPCharacter OtherActor))
  (if (Utilities|Enum|Equal(Enum) (Networking|GetLocalRole _asppcharacter) "ROLE_Authority")
    (Class|PPMonsterTrigger|OnPlayerin _asppcharacter)
    (Development|PrintString "Hello In")))

(fn ConstructionScript)