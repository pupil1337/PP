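; Player controller that toggles the BP_ESC widget on screen when the ESC input action is pressed.
; Each opening press creates a new widget, stores it, adds it to the viewport and shows the mouse cursor.
; The alternate press removes the stored widget from its parent and hides the cursor.
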(event Input|ActionEvents|InputActionESC
  (params (Key :type Key%20Structure :default "None"))
  (bind _self self)
  (:Pressed
    (bind _output_get (Variables|Default|SetbTips (not (Variables|Default|GetbTips))))
    (if _output_get
      (bind _returnvalue (UserInterface|CreateWidget "/Game/BP/UI/BP_ESC.BP_ESC_C" _self))
      (bind _output_get_2 (Variables|Default|SetTips _returnvalue))
      (UserInterface|Viewport|AddtoViewport _output_get_2 0)
      (Variables|Default|SetbShowMouseCursor _self true)
      (else
        (Widget|RemovefromParent (Variables|Default|GetTips))
        (Variables|Default|SetbShowMouseCursor false)))))

(fn ConstructionScript)